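; Menu game mode for an alphabet-finding game that shows either the start screen or the ranking screen on BeginPlay.
; The IsGameEnd flag on GI_FindAlphabet selects UI_Ranking when set, otherwise UI_GameStart, then enables the mouse cursor and UI-only input.
; LoadScoreData reads GameResultArray from the BP_RankData save slot to feed the ranking widget, with no check for a missing save.
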(event `self.ReceiveBeginPlay`
  (bind _returnvalue (`GameplayStatics.GetPlayerController` 0))
  (if (`/Game/BluePrints/GI_FindAlphabet.IsGameEnd` (cast `/Game/BluePrints/GI_FindAlphabet` (`GameplayStatics.GetGameInstance`) :!pure true))
    (bind _returnstring (`self.LoadScoreData`))
    (bind _returnvalue_2 (`|CreateWidget` "/Game/UI/UI_Ranking.UI_Ranking_C" _returnvalue _returnstring))
    (`UserWidget.AddToViewport` _returnvalue_2 0)
    (set `PlayerController.bShowMouseCursor` true _returnvalue)
    (`WidgetBlueprintLibrary.SetInputMode_UIOnlyEx` _returnvalue _returnvalue_2)
    (else
      (bind _returnvalue_3 (`|CreateWidget` "/Game/UI/UI_GameStart.UI_GameStart_C" _returnvalue))
      (`UserWidget.AddToViewport` _returnvalue_3 0)
      (set `PlayerController.bShowMouseCursor` true _returnvalue)
      (`WidgetBlueprintLibrary.SetInputMode_UIOnlyEx` _returnvalue _returnvalue_3))))

(fn `LoadScoreData`
  (returns (ReturnString :type "Array of /Game/BluePrints/BP_GameResultStructure Structure"))
  (bind _returnvalue (`GameplayStatics.LoadGameFromSlot` (`self.Slot Name`)))
  (return (`/Game/BluePrints/BP_RankData.GameResultArray` (cast `/Game/BluePrints/BP_RankData` _returnvalue :!pure true))))

(fn `UserConstructionScript`)