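; Game mode for a timed find-the-alphabet shooting game, setting up HUD widgets, Enhanced Input and the bullet count.
; Tick counts toward the time limit, while HitAlphabet records found letters and declares victory at two.
; GameEnd pauses, scores by outcome, appends player name and score to a BP_RankData save, then shows the victory or game-over UI.
; StartTimer is an alternative timeout, not called within this Blueprint.
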(event `self.ReceiveBeginPlay`
  (`WidgetBlueprintLibrary.SetInputMode_GameOnly` (`GameplayStatics.GetPlayerController` 0))
  (bind _returnvalue (`|CreateWidget` "/Game/UI/UI_Aimingpoint.UI_Aimingpoint_C"))
  (bind _returnvalue_2 (`|CreateWidget` "/Game/UI/UI_Bullet.UI_Bullet_C"))
  (bind _returnvalue_3 (`|CreateWidget` "/Game/UI/UI_Timer.UI_Timer_C"))
  (`UserWidget.AddToViewport` _returnvalue_2 0)
  (`UserWidget.AddToViewport` _returnvalue 0)
  (`UserWidget.AddToViewport` _returnvalue_3 0)
  (set `self.BulletCount` 30)
  (`EnhancedInputSubsystemInterface.AddMappingContext` (pcsubsystem `EnhancedInputLocalPlayerSubsystem` (`GameplayStatics.GetPlayerController` 0)) "/Game/Preset/Input/IMC_Main.IMC_Main" 0 (struct)))

(event `self.ReceiveTick`
  (params (DeltaSeconds :type "Float (single-precision)"))
  (if (>= (`self.CurrentTime`) (`self.LimitTime`))
    (`self.GameEnd` "NewEnumerator0" (`KismetMathLibrary.FTrunc` (`self.LimitTime`)) (`self.BulletCount`))
    (else
      (set `self.CurrentTime` (+ (`self.CurrentTime`) DeltaSeconds)))))

(fn `Calculate Score`
  (params (GameEndStatus :type "/Game/BluePrints/E_GameEndStatus Enum" :default "NewEnumerator0") (ClearTime :type Integer) (LeftBulletCount :type Integer) (FoundAlphabetCount :type Integer))
  (returns (Score :type Integer))
  (locals (NewScore :type Integer))
  (switch `/Game/BluePrints/E_GameEndStatus` GameEndStatus
    (:`NewEnumerator0`
      (bind _output_get (set `local.NewScore` (* 100 FoundAlphabetCount) :!label _label)))
    (:`NewEnumerator1`
      (goto _label))
    (:`NewEnumerator2`
      (set `local.NewScore` (+ (`local.NewScore`) 1000 (* ClearTime 10) (* LeftBulletCount 10)))))
  (return _output_get))

(fn `GameEnd`
  (params (GameEndStatus :type "/Game/BluePrints/E_GameEndStatus Enum" :default "NewEnumerator0") (ClearTime :type Integer) (LeftBulletCount :type Integer))
  (bind _returnvalue (`GameplayStatics.GetPlayerController` 0))
  (`GameplayStatics.SetGamePaused` true)
  (bind _score (`self.Calculate Score` GameEndStatus ClearTime LeftBulletCount (`KismetArrayLibrary.Array_Length` (`self.FoundAlphabetArray`))))
  (`self.SaveScoreData` (`/Game/BluePrints/GI_FindAlphabet.PlayerName` (cast `/Game/BluePrints/GI_FindAlphabet` (`GameplayStatics.GetGameInstance`) :!pure true)) _score)
  (switch `/Game/BluePrints/E_GameEndStatus` GameEndStatus
    (:`NewEnumerator0`
      (set `self.GameEndWidgetClass` "/Game/UI/UI_GameOver.UI_GameOver_C" :!label _label))
    (:`NewEnumerator1`
      (goto _label))
    (:`NewEnumerator2`
      (set `self.GameEndWidgetClass` "/Game/UI/UI_Victory.UI_Victory_C")))
  (bind _returnvalue_2 (`|CreateWidget` (`self.GameEndWidgetClass`)))
  (`UserWidget.AddToViewport` _returnvalue_2 0)
  (set `PlayerController.bShowMouseCursor` true _returnvalue)
  (`WidgetBlueprintLibrary.SetInputMode_UIOnlyEx` _returnvalue _returnvalue_2)
  (set `/Game/BluePrints/GI_FindAlphabet.IsGameEnd` true (cast `/Game/BluePrints/GI_FindAlphabet` (`GameplayStatics.GetGameInstance`) :!pure true)))

(fn `HitAlphabet`
  (params (HitActor :type "/Game/BluePrints/BP_Alphabet Object Reference"))
  (`KismetSystemLibrary.PrintString` "You Found Alphabet!" true true (struct :`R` 0.068019 :`G` 1.0 :`A` 1.0) 10.0)
  (`KismetArrayLibrary.Array_Add` (`self.FoundAlphabetArray`) (`/Game/BluePrints/BP_Alphabet.AlphabetIndex` HitActor))
  (if (== (`KismetArrayLibrary.Array_Length` (`self.FoundAlphabetArray`)) 2)
    (`self.GameEnd` "NewEnumerator2" (`KismetMathLibrary.FTrunc` (`self.CurrentTime`)) (`self.BulletCount`))))

(fn `HitOtherActor`
  (`KismetSystemLibrary.PrintString` "This Is Not Alphabet!" true true (struct :`R` 1.0 :`B` 0.095176 :`A` 1.0)))

(fn `SaveScoreData`
  (params (Name :type String) (Score :type Integer))
  (locals (NewScoreData :type "Array of String") (NewResultArray :type "Array of /Game/BluePrints/BP_GameResultStructure Structure"))
  (bind _saveslotname (`self.SaveSlotName`))
  (bind _saveslotname_2 (`self.SaveSlotName`))
  (bind _returnvalue (`GameplayStatics.DoesSaveGameExist` _saveslotname_2))
  (if _returnvalue
    (bind _returnvalue_2 (`GameplayStatics.LoadGameFromSlot` _saveslotname_2))
    (bind _output_get (set `self.SaveDataInstance` (cast `/Game/BluePrints/BP_RankData` _returnvalue_2 :!pure true)))
    (`KismetArrayLibrary.Array_Add` (`/Game/BluePrints/BP_RankData.GameResultArray` _output_get) (make `/Game/BluePrints/BP_GameResultStructure` Name Score))
    (`GameplayStatics.SaveGameToSlot` _output_get _saveslotname)
    (else
      (bind _returnvalue_3 (`GameplayStatics.CreateSaveGameObject` "/Game/BluePrints/BP_RankData.BP_RankData_C"))
      (bind _output_get_2 (set `self.SaveDataInstance` _returnvalue_3))
      (`KismetArrayLibrary.Array_Add` (`local.NewResultArray`) (make `/Game/BluePrints/BP_GameResultStructure` Name Score))
      (set `/Game/BluePrints/BP_RankData.GameResultArray` (`local.NewResultArray`) _output_get_2)
      (`GameplayStatics.SaveGameToSlot` _output_get_2 _saveslotname))))

(fn `Start Timer`
  (`KismetSystemLibrary.K2_SetTimer` null "GameEnd" (`self.LimitTime`)))

(fn `UserConstructionScript`)