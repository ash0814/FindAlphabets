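; Actor Blueprint that displays a single 3D letter mesh chosen by its AlphabetIndex value.
; The Construction Script switches on the index and assigns the matching A to Z static mesh to AlphabetStaticMesh, so the letter updates in the editor.
; Any index outside that range falls back to the SM_AVP2_0 mesh.
; The event graph holds only empty event stubs, so there is no runtime logic.
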(event `self.ReceiveActorBeginOverlap`
  (params (OtherActor :type "Actor Object Reference")))

(fn `UserConstructionScript`
  (bind _alphabetstaticmesh (`self.AlphabetStaticMesh`))
  (switch `int` (`self.AlphabetIndex`)
    (:`Default`
      (`StaticMeshComponent.SetStaticMesh` (`self.AlphabetStaticMesh`) "/Game/ArchVisPolishPack02/Meshes/Numbers/SM_AVP2_0.SM_AVP2_0"))
    (:`0`
      (`StaticMeshComponent.SetStaticMesh` _alphabetstaticmesh "/Game/ArchVisPolishPack02/Meshes/Letters/SM_AVP2_A.SM_AVP2_A"))
    (:`1`
      (`StaticMeshComponent.SetStaticMesh` _alphabetstaticmesh "/Game/ArchVisPolishPack02/Meshes/Letters/SM_AVP2_B.SM_AVP2_B"))
    (:`2`
      (`StaticMeshComponent.SetStaticMesh` _alphabetstaticmesh "/Game/ArchVisPolishPack02/Meshes/Letters/SM_AVP2_C.SM_AVP2_C"))
    (:`3`
      (`StaticMeshComponent.SetStaticMesh` _alphabetstaticmesh "/Game/ArchVisPolishPack02/Meshes/Letters/SM_AVP2_D.SM_AVP2_D"))
    (:`4`
      (`StaticMeshComponent.SetStaticMesh` _alphabetstaticmesh "/Game/ArchVisPolishPack02/Meshes/Letters/SM_AVP2_E.SM_AVP2_E"))
    (:`5`
      (`StaticMeshComponent.SetStaticMesh` _alphabetstaticmesh "/Game/ArchVisPolishPack02/Meshes/Letters/SM_AVP2_F.SM_AVP2_F"))
    (:`6`
      (`StaticMeshComponent.SetStaticMesh` _alphabetstaticmesh "/Game/ArchVisPolishPack02/Meshes/Letters/SM_AVP2_G.SM_AVP2_G"))
    (:`7`
      (`StaticMeshComponent.SetStaticMesh` _alphabetstaticmesh "/Game/ArchVisPolishPack02/Meshes/Letters/SM_AVP2_H.SM_AVP2_H"))
    (:`8`
      (`StaticMeshComponent.SetStaticMesh` _alphabetstaticmesh "/Game/ArchVisPolishPack02/Meshes/Letters/SM_AVP2_I.SM_AVP2_I"))
    (:`9`
      (`StaticMeshComponent.SetStaticMesh` _alphabetstaticmesh "/Game/ArchVisPolishPack02/Meshes/Letters/SM_AVP2_J.SM_AVP2_J"))
    (:`10`
      (`StaticMeshComponent.SetStaticMesh` _alphabetstaticmesh "/Game/ArchVisPolishPack02/Meshes/Letters/SM_AVP2_K.SM_AVP2_K"))
    (:`11`
      (`StaticMeshComponent.SetStaticMesh` _alphabetstaticmesh "/Game/ArchVisPolishPack02/Meshes/Letters/SM_AVP2_L.SM_AVP2_L"))
    (:`12`
      (`StaticMeshComponent.SetStaticMesh` _alphabetstaticmesh "/Game/ArchVisPolishPack02/Meshes/Letters/SM_AVP2_M.SM_AVP2_M"))
    (:`13`
      (`StaticMeshComponent.SetStaticMesh` _alphabetstaticmesh "/Game/ArchVisPolishPack02/Meshes/Letters/SM_AVP2_N.SM_AVP2_N"))
    (:`14`
      (`StaticMeshComponent.SetStaticMesh` _alphabetstaticmesh "/Game/ArchVisPolishPack02/Meshes/Letters/SM_AVP2_O.SM_AVP2_O"))
    (:`15`
      (`StaticMeshComponent.SetStaticMesh` _alphabetstaticmesh "/Game/ArchVisPolishPack02/Meshes/Letters/SM_AVP2_P.SM_AVP2_P"))
    (:`16`
      (`StaticMeshComponent.SetStaticMesh` _alphabetstaticmesh "/Game/ArchVisPolishPack02/Meshes/Letters/SM_AVP2_Q.SM_AVP2_Q"))
    (:`17`
      (`StaticMeshComponent.SetStaticMesh` _alphabetstaticmesh "/Game/ArchVisPolishPack02/Meshes/Letters/SM_AVP2_R.SM_AVP2_R"))
    (:`18`
      (`StaticMeshComponent.SetStaticMesh` _alphabetstaticmesh "/Game/ArchVisPolishPack02/Meshes/Letters/SM_AVP2_S.SM_AVP2_S"))
    (:`19`
      (`StaticMeshComponent.SetStaticMesh` _alphabetstaticmesh "/Game/ArchVisPolishPack02/Meshes/Letters/SM_AVP2_T.SM_AVP2_T"))
    (:`20`
      (`StaticMeshComponent.SetStaticMesh` _alphabetstaticmesh "/Game/ArchVisPolishPack02/Meshes/Letters/SM_AVP2_U.SM_AVP2_U"))
    (:`21`
      (`StaticMeshComponent.SetStaticMesh` _alphabetstaticmesh "/Game/ArchVisPolishPack02/Meshes/Letters/SM_AVP2_V.SM_AVP2_V"))
    (:`22`
      (`StaticMeshComponent.SetStaticMesh` _alphabetstaticmesh "/Game/ArchVisPolishPack02/Meshes/Letters/SM_AVP2_W.SM_AVP2_W"))
    (:`23`
      (`StaticMeshComponent.SetStaticMesh` _alphabetstaticmesh "/Game/ArchVisPolishPack02/Meshes/Letters/SM_AVP2_X.SM_AVP2_X"))
    (:`24`
      (`StaticMeshComponent.SetStaticMesh` _alphabetstaticmesh "/Game/ArchVisPolishPack02/Meshes/Letters/SM_AVP2_Y.SM_AVP2_Y"))
    (:`25`
      (`StaticMeshComponent.SetStaticMesh` _alphabetstaticmesh "/Game/ArchVisPolishPack02/Meshes/Letters/SM_AVP2_Z.SM_AVP2_Z"))))