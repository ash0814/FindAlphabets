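; BP_Bullet is a projectile that moves forward each Tick and reports hits on BP_Alphabet actors to BP_GameModeBase.
; An overlap calls HitAlphabet and destroys the letter, or calls HitOtherActor, then explodes, destroys the bullet and calls GameEnd if no bullets remain.
; A three-second Delay on Tick feeds the same miss path as a lifetime limit.
; An uncalled helper extracts a letter from an actor's display name.
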(event `self.ReceiveActorBeginOverlap`
  (params (OtherActor :type "Actor Object Reference"))
  (bind _asbp_game_mode_base (cast `/Game/BluePrints/BP_GameModeBase` (`GameplayStatics.GetGameMode`) :!pure true))
  (bind _asbp_alphabet (cast `/Game/BluePrints/BP_Alphabet` OtherActor)
    (:`then`
      (`/Game/BluePrints/BP_GameModeBase.HitAlphabet` (cast `/Game/BluePrints/BP_GameModeBase` (`GameplayStatics.GetGameMode`) :!pure true) _asbp_alphabet)
      (`self.K2_DestroyActor` _asbp_alphabet))
    (:`CastFailed`
      (`/Game/BluePrints/BP_GameModeBase.HitOtherActor` (cast `/Game/BluePrints/BP_GameModeBase` (`GameplayStatics.GetGameMode`) :!pure true) :!label _label)))
  (`GameplayStatics.SpawnEmitterAtLocation` "/Game/StarterContent/Particles/P_Explosion.P_Explosion" (`self.K2_GetActorLocation`))
  (`self.K2_DestroyActor`)
  (if (<= (`/Game/BluePrints/BP_GameModeBase.BulletCount` _asbp_game_mode_base) 0)
    (`/Game/BluePrints/BP_GameModeBase.GameEnd` _asbp_game_mode_base "NewEnumerator1" (`KismetMathLibrary.FTrunc` (`/Game/BluePrints/BP_GameModeBase.CurrentTime` _asbp_game_mode_base)) (`/Game/BluePrints/BP_GameModeBase.BulletCount` _asbp_game_mode_base))))

(event `self.ReceiveTick`
  (params (DeltaSeconds :type "Float (single-precision)"))
  ;[1 1 1] Bullet Move - Destroy After 3 sec
  (`self.K2_SetActorLocation` (+ (`self.K2_GetActorLocation`) (* (`self.GetActorForwardVector`) DeltaSeconds (`self.MoveSpeed`))))
  (`KismetSystemLibrary.Delay` 3.0)
  (goto _label))

(fn `ConvertDisplayNameToAlphabet`
  (params (HitAlphabetObject :type "/Game/BluePrints/BP_Alphabet Object Reference"))
  (returns (AlphabetName :type String))
  (bind _returnvalue (`KismetSystemLibrary.GetDisplayName` HitAlphabetObject))
  (`KismetSystemLibrary.PrintString` _returnvalue true true (struct :`R` 0.072297 :`G` 0.260417 :`A` 1.0) 10.0)
  (return (`KismetStringLibrary.GetSubstring` _returnvalue 12)))

(fn `UserConstructionScript`)