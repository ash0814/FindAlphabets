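; BP_Player is the first-person-style player character that moves, looks, jumps, shoots and shows a found-alphabets overlay.
; Enhanced Input from IMC_Main drives movement, look, shooting and the hold-to-view UI_FoundAlphabets widget, while raw keys handle jump and right-mouse FOV zoom.
; Shooting checks and decrements BulletCount on BP_GameModeBase, then spawns BP_Bullet at the camera's transform.
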(event `EnhancedInput|/Game/Preset/Input/IA/IA_FCheckAlphabets`
  (params (ActionValue :type Boolean) (ElapsedSeconds :type "Float (double-precision)") (TriggeredSeconds :type "Float (double-precision)") (InputAction :type "InputAction Object Reference" :default "/Game/Preset/Input/IA/IA_FCheckAlphabets.IA_FCheckAlphabets"))
  (:`Started`
    (bind _returnvalue (`|CreateWidget` "/Game/UI/UI_FoundAlphabets.UI_FoundAlphabets_C" (`GameplayStatics.GetPlayerController` 0)))
    (set `self.FoundAlphabetWidget` _returnvalue)
    (`UserWidget.AddToViewport` _returnvalue 0))
  (:`Completed`
    (`Widget.RemoveFromParent` (`self.FoundAlphabetWidget`))))

(event `self.ReceiveBeginPlay`
  (`EnhancedInputSubsystemInterface.AddMappingContext` (pcsubsystem `EnhancedInputLocalPlayerSubsystem` (`GameplayStatics.GetPlayerController` 0)) "/Game/Preset/Input/IMC_Main.IMC_Main" 0 (struct)))

(event `EnhancedInput|/Game/Preset/Input/IA/IA_FMove`
  (params (ActionValue :type "Vector2D Structure") (ElapsedSeconds :type "Float (double-precision)") (TriggeredSeconds :type "Float (double-precision)") (InputAction :type "InputAction Object Reference" :default "/Game/Preset/Input/IA/IA_FMove.IA_FMove"))
  (bind _returnvalue (`self.GetControlRotation`))
  (:`Triggered`
    (`|ExecutionSequence` :!label _label
      (:`then_0`
        (`self.AddMovementInput` (`KismetMathLibrary.GetForwardVector` _returnvalue) ActionValue_Y))
      (:`then_1`
        (`self.AddMovementInput` (`KismetMathLibrary.GetRightVector` _returnvalue) ActionValue_X))))
  (:`Completed`
    (goto _label)))

(event `EnhancedInput|/Game/Preset/Input/IA/IA_FLook`
  (params (ActionValue :type "Vector2D Structure") (ElapsedSeconds :type "Float (double-precision)") (TriggeredSeconds :type "Float (double-precision)") (InputAction :type "InputAction Object Reference" :default "/Game/Preset/Input/IA/IA_FLook.IA_FLook"))
  (:`Triggered`
    (`self.AddControllerPitchInput` ActionValue_Y)
    (`self.AddControllerYawInput` ActionValue_X)))

(event `Key|SpaceBar`
  (params (Key :type "Key Structure"))
  (:`Pressed`
    (`self.Jump`)))

(event `EnhancedInput|/Game/Preset/Input/IA/IA_FShoot`
  (params (ActionValue :type Boolean) (ElapsedSeconds :type "Float (double-precision)") (TriggeredSeconds :type "Float (double-precision)") (InputAction :type "InputAction Object Reference" :default "/Game/Preset/Input/IA/IA_FShoot.IA_FShoot"))
  (bind _asbp_game_mode_base (cast `/Game/BluePrints/BP_GameModeBase` (`GameplayStatics.GetGameMode`) :!pure true))
  (:`Started`
    (if (> (`/Game/BluePrints/BP_GameModeBase.BulletCount` _asbp_game_mode_base) 0)
      (`/Engine/EditorBlueprintResources/StandardMacros.DecrementInt` (`/Game/BluePrints/BP_GameModeBase.BulletCount` _asbp_game_mode_base)
        (:`  `
          (`|SpawnActorFromClass` "/Game/BluePrints/BP_Bullet.BP_Bullet_C" (`SceneComponent.K2_GetComponentToWorld` (`self.Camera`)) "Undefined" "MultiplyWithRoot" null null))))))

(event `Key|RightMouseButton`
  (params (Key :type "Key Structure"))
  (bind _camera (`self.Camera`))
  (:`Pressed`
    (`CameraComponent.SetFieldOfView` _camera 50.0))
  (:`Released`
    (`CameraComponent.SetFieldOfView` _camera 90.0)))

(fn `UserConstructionScript`)